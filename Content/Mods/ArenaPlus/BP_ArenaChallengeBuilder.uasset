(fn `AddEnemyToWave`
  (params (EnemyName :type String) (Amount :type Integer :default 1))
  (returns (Builder :type "/Game/Mods/ArenaPlus/BP_ArenaChallengeBuilder Object Reference"))
  (bind _enemyamounts (`self.GetCurrentWaveEnemyAmounts`)
    (:`OutExec`
      (bind (_value _returnvalue) (`BlueprintMapLibrary.Map_Find` _enemyamounts EnemyName))
      (if _returnvalue
        (`BlueprintMapLibrary.Map_Add` _enemyamounts EnemyName (+ _value Amount))
        (else
          (`BlueprintMapLibrary.Map_Add` _enemyamounts EnemyName Amount)))
      (return self))))

(fn `Build`
  (returns (Builder :type "/Game/Mods/ArenaPlus/BP_ArenaChallengeBuilder Object Reference") (ArenaChallenge :type "/Game/Mods/ArenaPlus/STR_ArenaChallenge Structure"))
  (locals (TempEnemyWaves :type "Array of /Game/Mods/ArenaPlus/STR_EnemyWave Structure"))
  (for _array_element (`self.Waves`)
    (bind (_enemywave _isvalidwave) (`self.BuildWave` _array_element))
    (if _isvalidwave
      (`KismetArrayLibrary.Array_Add` (`local.TempEnemyWaves`) _enemywave)))
  (return self (make `/Game/Mods/ArenaPlus/STR_ArenaChallenge` (`local.TempEnemyWaves`))))

(fn `BuildWave`
  (params (BuilderWave :type "/Game/Mods/ArenaPlus/STR_ArenaBuilderWave Structure"))
  (returns (EnemyWave :type "/Game/Mods/ArenaPlus/STR_EnemyWave Structure") (IsValidWave :type Boolean))
  (locals (TempEnemySpawns :type "Array of /Game/Mods/ArenaPlus/STR_EnemySpawn Structure") (TempIsValid :type Boolean))
  (bind _enemyamounts (break `/Game/Mods/ArenaPlus/STR_ArenaBuilderWave` BuilderWave))
  (set `self.CurrentRaisedSpawnIndex` 0)
  (bind _keys (`BlueprintMapLibrary.Map_Keys` _enemyamounts))
  (for _array_element _keys
    (bind _value (`BlueprintMapLibrary.Map_Find` _enemyamounts _array_element))
    (bind _spawnlocations (`self.GetSpawnLocations` _array_element _value))
    (`KismetArrayLibrary.Array_Add` (`local.TempEnemySpawns`) (make `/Game/Mods/ArenaPlus/STR_EnemySpawn` _array_element _value _spawnlocations))
    (if (> _value 0)
      (set `local.TempIsValid` true)))
  (return (make `/Game/Mods/ArenaPlus/STR_EnemyWave` (`local.TempEnemySpawns`)) (`local.TempIsValid`)))

(fn `DetermineNextSpawnLocation`
  (params (EnemyName :type String))
  (returns (SpawnLocation :type "SpawnLocation Object Reference"))
  (locals (TempSpawnLocation :type "SpawnLocation Object Reference"))
  (bind _supportsraisedspawn (`/Game/Mods/ArenaPlus/BPF_ArenaHelpers.DoesEnemySupportRaisedSpawn` EnemyName))
  (if _supportsraisedspawn
    (if (`KismetArrayLibrary.Array_IsValidIndex` (`self.RaisedSpawnLocations`) (`self.CurrentRaisedSpawnIndex`))
      (set `local.TempSpawnLocation` (`|GetArrayItem` (`self.RaisedSpawnLocations`) (`self.CurrentRaisedSpawnIndex`)))
      (`/Engine/EditorBlueprintResources/StandardMacros.IncrementInt` (`self.CurrentRaisedSpawnIndex`)
        (:`  `
          _))
      (else
        (if (not (`KismetArrayLibrary.Array_IsValidIndex` (`self.GroundedSpawnLocations`) (`self.CurrentGroundedSpawnIndex`))) :!label _label
          (set `self.CurrentGroundedSpawnIndex` 0))
        (set `local.TempSpawnLocation` (`|GetArrayItem` (`self.GroundedSpawnLocations`) (`self.CurrentGroundedSpawnIndex`)))
        (`/Engine/EditorBlueprintResources/StandardMacros.IncrementInt` (`self.CurrentGroundedSpawnIndex`)
          (:`  `
            _))))
    (else
      (goto _label)))
  (return (`local.TempSpawnLocation`)))

(fn `GetSpawnLocations`
  (params (EnemyName :type String) (Amount :type Integer))
  (returns (SpawnLocations :type "Array of SpawnLocation Object Reference"))
  (locals (TempSpawnLocations :type "Array of SpawnLocation Object Reference"))
  (for _ (range 1 (+ Amount 1))
    (bind _spawnlocation (`self.DetermineNextSpawnLocation` EnemyName))
    (`KismetArrayLibrary.Array_Add` (`local.TempSpawnLocations`) _spawnlocation))
  (return (`local.TempSpawnLocations`)))

(fn `NextWave`
  (returns (Builder :type "/Game/Mods/ArenaPlus/BP_ArenaChallengeBuilder Object Reference"))
  (`/Engine/EditorBlueprintResources/StandardMacros.IncrementInt` (`self.CurrentWaveIndex`)
    (:`  `
      (return self))))

(fn `PreviousWave`
  (returns (Builder :type "/Game/Mods/ArenaPlus/BP_ArenaChallengeBuilder Object Reference"))
  (bind _result (`/Engine/EditorBlueprintResources/StandardMacros.DecrementInt` (`self.CurrentWaveIndex`))
    (:`  `
      (if (< _result 0)
        (set `self.CurrentWaveIndex` 0)
        (return self)))))

(fn `UserConstructionScript`)