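; BP_Wave_DOV is an ArenaPlus mod wave Blueprint that assembles the enemy spawn data for an arena wave.
; AddEnemyToSpawn converts each enemy entry into a name-keyed SpawnGroups entry with its locations and fixed count, plus a matching ItemsToSpawn selection of type EnemyDefinition.
; Two debug helpers report the item count and group keys through the empty PrintToModLoader event.
; BeginPlay and the construction script are empty.
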(event `PrintToModLoader`
  (params (Message :type String)))

(event `self.ReceiveBeginPlay`)

(fn `Add Enemy to Spawn`
  (params (EnemySpawn :type "/Game/Mods/ArenaPlus/STR_EnemySpawn Structure"))
  (bind (_name _amount _spawnlocations) (break `/Game/Mods/ArenaPlus/STR_EnemySpawn` EnemySpawn))
  (bind _negativeoneperplatformint (`self.NegativeOnePerPlatformInt`))
  (`BlueprintMapLibrary.Map_Add` (`self.SpawnGroups`) (`KismetStringLibrary.Conv_StringToName` _name) (make `DynamicObjectGroupInfo` (struct) (struct) false false false false false _spawnlocations _amount _amount _negativeoneperplatformint _negativeoneperplatformint 0.1 0.1 1.0 false false false true true "AdjustIfPossibleButAlwaysSpawn" false 10000.0 5000.0 3.0 1 1.0 false "None" "Wander" false (struct) false (struct) "HBT_Count"))
  (`KismetArrayLibrary.Array_Add` (`self.ItemsToSpawn`) (make `SpawnSelectInfo` :`ObjectType` "EnemyDefinition" :`ObjectToSpawn` _name :`MyIndex` (`KismetArrayLibrary.Array_Length` (`self.ItemsToSpawn`)) :`GroupName` _name)))

(fn `UserConstructionScript`)