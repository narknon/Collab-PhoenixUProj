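; ArenaPlus mod manager actor that streams in a custom arena map when an arena level's wave spawner appears.
; A throttled Tick polls for BP_WaveSpawner within the arena level, as a workaround for lacking an arena entry event.
; Detection passes a DoOnce that resets after a delay, then loads M_ArenaMap as a level instance at the spawner's location, removing any previous instance.
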(event `OnWaveSpawnerDetected`
  (params (WaveSpawner :type "/Game/Gameplay/BluePrints/Universal/BP_WaveSpawner Object Reference"))
  (`/Engine/EditorBlueprintResources/StandardMacros.DoOnce` false :!label _label
    (:`Completed`
      (`self.LoadArena` (`self.K2_GetActorLocation` WaveSpawner))
      (`KismetSystemLibrary.Delay` 3.0)
      (goto _label :!via `Reset`))))

(event `self.ReceiveTick`
  (params (DeltaSeconds :type "Float (single-precision)"))
  (bind (_wavespawner _found) (`self.FindWaveSpawner`)) ; A Wave Spawner exists whenever an arena level is loaded (on initiation and on retry)
  (if _found
    (bind _returnvalue (`/Game/Mods/ArenaPlus/BPF_ArenaHelpers.IsActorWithinArenaLevel` _wavespawner))
    (if _returnvalue
      (`self.OnWaveSpawnerDetected` _wavespawner))))

(event `PrintToModLoader`
  (params (Message :type String)))

(event `self.ReceiveBeginPlay`)

(fn `FindWaveSpawner`
  (returns (WaveSpawner :type "/Game/Gameplay/BluePrints/Universal/BP_WaveSpawner Object Reference") (Found :type Boolean))
  (bind _returnvalue (`GameplayStatics.GetActorOfClass` "/Game/Gameplay/BluePrints/Universal/BP_WaveSpawner.BP_WaveSpawner_C"))
  (return _returnvalue (`KismetSystemLibrary.IsValid` _returnvalue)))

(fn `LoadArena`
  (params (Location :type "Vector Structure"))
  (bind _arenalevelinstance (`self.ArenaLevelInstance`))
  (if (`KismetSystemLibrary.IsValid` _arenalevelinstance)
    (`LevelStreaming.SetIsRequestingUnloadAndRemoval` _arenalevelinstance true))
  (bind (_boutsuccess _returnvalue) (`LevelStreamingDynamic.LoadLevelInstanceBySoftObjectPtr` "/Game/Mods/ArenaPlus/M_ArenaMap.M_ArenaMap" Location))
  (set `self.ArenaLevelInstance` _returnvalue))

(fn `UnloadArena`
  (if (`KismetSystemLibrary.IsValid` (`self.ArenaLevelInstance`))
    (`LevelStreaming.SetIsRequestingUnloadAndRemoval` (`self.ArenaLevelInstance`) true)
    (set `self.ArenaLevelInstance` null)))

(fn `UserConstructionScript`)